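; BPFL_WaveUtils is a Blueprint function library of helpers for combining and creating wave data.
; OverlapWaves merges an array of waves into one frequency and amplitude, averaging frequencies after scaling each by 100 and summing amplitudes, with zeros for an empty array.
; GetWavesFromStruct converts an array of initial wave structs into BP_Wave objects constructed under a supplied Outer.
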(fn OverlapWaves
  (params (Waves :type Array%20of%20BP%20Wave%20Object%20References))
  (if (== (Utilities|Array|Length Waves) 0)
    (return 0.0 0.0)
    (else
      (for _array_element Waves
        (LocalVariables|SetTotFrequency (+ (* (Variables|/Game/Blueprints/Core/Wave/BP_Wave.BP_Wave_C|GetFrequency _array_element) 1e+02) (LocalVariables|GetTotFrequency)))
        (LocalVariables|SetTotAmplitude (+ (Variables|/Game/Blueprints/Core/Wave/BP_Wave.BP_Wave_C|GetAmplitude _array_element) (LocalVariables|GetTotAmplitude))))
      (return (/ (LocalVariables|GetTotFrequency) (Utilities|Array|Length Waves)) (LocalVariables|GetTotAmplitude)))))

(fn GetWavesfromStruct
  (params (Initial%20Waves :type Array%20of%20S%20Wave%20Structures) (Outer :type Object%20Object%20Reference))
  (for _array_element Initial%20Waves
    (bind _returnvalue (Game|ConstructObjectfromClass Outer "/Game/Blueprints/Core/Wave/BP_Wave.BP_Wave_C" (.Frequency (Utilities|Struct|BreakS_Wave _array_element)) (.Amplitude (Utilities|Struct|BreakS_Wave _array_element))))
    (Utilities|Array|Add (LocalVariables|GetWaves) _returnvalue))
  (return (LocalVariables|GetWaves)))