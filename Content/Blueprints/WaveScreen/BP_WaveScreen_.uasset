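; BP_WaveScreen is a screen actor that displays a set of waves through a material on its plane mesh.
; On BeginPlay it creates a dynamic instance of MI_WaveScreen and applies it to Plane1.
; Update zeroes all 30 numbered Frequency and Amplitude parameter pairs, then writes each incoming wave into the pair matching its 1-based position.
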(event Custom|Event%20Update
  (params (Waves :type Array%20of%20BP%20Wave%20Object%20References))
  (CallFunction|ClearMaterialInstanceParameters)
  (CallFunction|SetMaterialInstanceParameters Waves))

(event EventBeginPlay
  (bind _returnvalue (Rendering|Material|CreateDynamicMaterialInstance (Variables|Default|GetPlane1) 0 "/Game/Blueprints/WaveScreen/MI_WaveScreen.MI_WaveScreen" "Screen" :!class /Script/Engine.PrimitiveComponent))
  (bind _output_get (Variables|Default|SetScreenMaterialInstance _returnvalue))
  (Rendering|Material|SetMaterial (Variables|Default|GetPlane1) 0 _output_get))

(fn ConstructionScript)

(fn ClearMaterialInstanceParameters
  (for _index (range 1 30)
    (Rendering|Material|SetScalarParameterValue (Variables|Default|GetScreenMaterialInstance) (Utilities|String|StringToName (Utilities|String|ToString(Text) (Utilities|Text|FormatText "Frequency{i}" _index))) 0.0 :!class /Script/Engine.MaterialInstanceDynamic)
    (Rendering|Material|SetScalarParameterValue (Variables|Default|GetScreenMaterialInstance) (Utilities|String|StringToName (Utilities|String|ToString(Text) (Utilities|Text|FormatText "Amplitude{i}" _index))) 0.0 :!class /Script/Engine.MaterialInstanceDynamic)))

(fn SetMaterialInstanceParameters
  (params (Waves :type Array%20of%20BP%20Wave%20Object%20References))
  (for (_array_element _array_index) Waves
    (Rendering|Material|SetScalarParameterValue (Variables|Default|GetScreenMaterialInstance) (Utilities|String|StringToName (Utilities|String|ToString(Text) (Utilities|Text|FormatText "Frequency{i}" (+ _array_index 1)))) (Variables|/Game/Blueprints/Core/Wave/BP_Wave.BP_Wave_C|GetFrequency _array_element) :!class /Script/Engine.MaterialInstanceDynamic)
    (Rendering|Material|SetScalarParameterValue (Variables|Default|GetScreenMaterialInstance) (Utilities|String|StringToName (Utilities|String|ToString(Text) (Utilities|Text|FormatText "Amplitude{i}" (+ _array_index 1)))) (Variables|/Game/Blueprints/Core/Wave/BP_Wave.BP_Wave_C|GetAmplitude _array_element) :!class /Script/Engine.MaterialInstanceDynamic)))