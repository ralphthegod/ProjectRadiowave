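; BP_CaptaScreen is a wave display screen that switches between an idle info view and an analyze view.
; Updates pass waves to the parent, then send their overlapped frequency and amplitude to the UI_WaveScreen widget.
; Analyze mode moves and rescales Plane1, swaps widget visibility and shows the combined values on UI_AnalyzeScreen.
; BeginPlay caches both widget references and hides the frequency field when the screen is disabled.
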(event Custom|Event%20Update
  (params (Waves :type Array%20of%20BP%20Wave%20Object%20References))
  (if (not (Variables|Default|GetIsAnalyzeMode?))
    (CallFunction|UpdateWaves Waves)))

(event Custom|Event%20Enable%20Analyze%20Mode
  (params (Waves :type Array%20of%20BP%20Wave%20Object%20References))
  ;[1 1 1] Analyze Mode
  (CallFunction|SetScreeninAnalyzeMode)
  (CallFunction|UpdateWaves Waves)
  (bind (_frequency _amplitude) (CallFunction|OverlapWaves Waves))
  (Default|EventShow (Variables|Default|GetAs%20UI%20Analyze%20Screen) _frequency _amplitude)
  (Rendering|SetVisibility (Variables|Default|GetAnalyzeWidget) true false)
  (Rendering|SetVisibility (Variables|Default|GetInfoWidget) false false))

(event Custom|Event%20Disable%20Analyze%20Mode
  (params (Waves :type Array%20of%20BP%20Wave%20Object%20References))
  ;[1 1 1] Analyze Mode
  (Variables|Default|SetIsAnalyzeMode? false)
  (Rendering|SetVisibility (Variables|Default|GetAnalyzeWidget) false true)
  (Rendering|SetVisibility (Variables|Default|GetInfoWidget) true false)
  (CallFunction|SetScreeninIdleMode)
  (CallFunction|EventUpdate Waves))

(event EventBeginPlay
  (|CallParentFunction)
  (|SetScreenDataVisibility))

(fn ConstructionScript)

(fn SetScreeninAnalyzeMode
  (bind _plane1 (Variables|Default|GetPlane1))
  (bind _returnvalue (Transformation|GetRelativeTransform _plane1))
  (bind (_location _rotation _scale) (Math|Transform|BreakTransform _returnvalue))
  (bind (_x _y _z) (Class|KismetMathLibrary|BreakVector3f _scale))
  (bind (_x_2 _y_2 _z_2) (Class|KismetMathLibrary|BreakVector3f _location))
  (Transformation|SetRelativeTransform _plane1 (Math|Transform|MakeTransform (Math|Vector|MakeVector _x_2 0.0 _z_2) _rotation (Math|Vector|MakeVector 0.075 _y _z)) false false))

(fn SetScreeninIdleMode
  (bind _plane1 (Variables|Default|GetPlane1))
  (bind _returnvalue (Transformation|GetRelativeTransform _plane1))
  (bind (_location _rotation _scale) (Math|Transform|BreakTransform _returnvalue))
  (bind (_x _y _z) (Class|KismetMathLibrary|BreakVector3f _scale))
  (bind (_x_2 _y_2 _z_2) (Class|KismetMathLibrary|BreakVector3f _location))
  (Transformation|SetRelativeTransform _plane1 (Math|Transform|MakeTransform (Math|Vector|MakeVector _x_2 1.6 _z_2) _rotation (Math|Vector|MakeVector 0.0425 _y _z)) false false))

(fn UpdateWaves
  (params (Waves :type Array%20of%20BP%20Wave%20Object%20References))
  (|CallParentFunction Waves)
  (bind (_frequency _amplitude) (CallFunction|OverlapWaves Waves))
  (Default|EventUpdate (Variables|Default|GetAs%20UI%20Wave%20Screen) Waves _frequency _amplitude))