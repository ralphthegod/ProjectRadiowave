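; Blueprint function library of generic utilities, holding one function meant to look up the display name of the key bound to an input action.
; The function gets player 0's player-mappable action key mappings and only prints their count to screen.
; The loop that matches the action and returns its key's short display name is disconnected, so the lookup never runs.
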(fn GetInputKeyNamebyActionMapping
  (params (Action :type Input%20Action%20Object%20Reference))
  (bind _returnvalue (Class|EnhancedInputSubsystemInterface|GetAllPlayerMappableActionKeyMappings(Message) (Game|GetPlayerController 0)))
  (Development|PrintString 0 (Utilities|String|ToString(Integer) (Utilities|Array|Length _returnvalue))))