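; BP_TriggerableDoor is a locked sci-fi door that opens once when it receives a Trigger event.
; On BeginPlay it spawns a BP_Screen showing configurable text, attaches it to a socket component, and labels its interaction widget "Locked Door".
; The first Trigger plays the door's skeletal mesh animation and tells the screen to show its unlock state.
; Highlight and Unhighlight toggle custom depth rendering on the mesh.
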(event EventBeginPlay
  (bind _returnvalue (Game|SpawnActorfromClass "/Game/Blueprints/TriggerableDoor/BP_Screen.BP_Screen_C" (Math|Conversions|ToTransform(Vector) "0, 0, 0") "Undefined" "MultiplyWithRoot" 0 (Variables|Default|GetTextToShow) 0))
  (bind _output_get (Variables|Default|SetScreen _returnvalue))
  (Transformation|AttachComponentToComponent _output_get (Variables|Default|GetScreenSocket1) "None" "SnapToTarget" "KeepRelative" "KeepWorld" true)
  (CallFunction|InitInteraction))

(event EventTrigger
  (Utilities|FlowControl|DoOnce false
    (:Completed
      (CallFunction|UnlockDoor)
      (Default|EventUnlock (Variables|Default|GetScreen)))))

(event EventHighlight
  (Rendering|SetRenderCustomDepth (Variables|Default|GetSkeletalMesh) true))

(event EventUnhighlight
  (Rendering|SetRenderCustomDepth (Variables|Default|GetSkeletalMesh) false))

(fn ConstructionScript)

(fn UnlockDoor
  (Components|Animation|PlayAnimation (Variables|Default|GetSkeletalMesh) "/Game/Meshes/Door/Cooper_SCIFI_DOOR11_Anim.Cooper_SCIFI_DOOR11_Anim" false))

(fn InitInteraction
  (bind _asui_info_on_screen (Utilities|Casting|CastToUI_InfoOnScreen (UserInterface|GetUserWidgetObject (Variables|Default|GetInteraction%20Label1))))
  (bind _output_get (Variables|Default|SetAs%20UI%20Info%20On%20Screen _asui_info_on_screen))
  (Default|EventSetText _output_get "Locked Door" "" (Utilities|Array|MakeArray)))