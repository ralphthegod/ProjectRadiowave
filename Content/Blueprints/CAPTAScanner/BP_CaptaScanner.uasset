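; CAPTA scanner that collects incoming waves and presents them on an attached screen and through an audio component.
; It spawns the screen onto the mesh's Screen socket and keeps a unique list of current waves.
; Outside analyze mode, changes redraw the screen and feed scaled frequencies to the speaker as harmonic multipliers.
; While analyzing, only changes from the analyzed source pass, toggling the screen's analyze mode.
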(event Custom|Event%20Receive%20New%20Waves
  (params (Waves :type Array%20of%20BP%20Wave%20Object%20References) (FromAnalyzed :type Boolean))
  (CallFunction|ReceiveNewWaves Waves)
  (Utilities|ShouldUpdate? FromAnalyzed
    (:From%20Analyzed
      (CallFunction|EventEnableAnalyzeMode Waves))
    (:then
      (CallFunction|UpdateScreen)
      (CallFunction|PlayWavesAudio))))

(event Custom|Event%20Stop%20Receiving%20Waves
  (params (Waves :type Array%20of%20BP%20Wave%20Object%20References) (FromAnalyzed :type Boolean))
  (CallFunction|StopReceivingWaves Waves)
  (Utilities|ShouldUpdate? FromAnalyzed
    (:From%20Analyzed
      (CallFunction|EventDisableAnalyzeMode))
    (:then
      (CallFunction|UpdateScreen)
      (CallFunction|PlayWavesAudio))))

(event Custom|Event%20Enable%20Analyze%20Mode
  (params (Waves :type Array%20of%20BP%20Wave%20Object%20References))
  (Default|EventEnableAnalyzeMode (Variables|Default|GetWaveScreen) Waves)
  (Variables|Default|SetAnalyzing true))

(event Custom|Event%20Disable%20Analyze%20Mode
  (Default|EventDisableAnalyzeMode (Variables|Default|GetWaveScreen) (Variables|Default|GetCurrentWaves))
  (Variables|Default|SetAnalyzing false))

(event EventBeginPlay
  (bind _returnvalue (Game|SpawnActorfromClass "/Game/Blueprints/WaveScreen/BP_CaptaScreen.BP_CaptaScreen_C" (Math|Conversions|ToTransform(Vector) "0, 0, 0") "Undefined" "MultiplyWithRoot" 0 0))
  (bind _output_get (Variables|Default|SetWaveScreen _returnvalue))
  (Transformation|AttachComponentToComponent _output_get (Variables|Default|GetStaticMesh) "Screen" "SnapToTarget" "KeepWorld" "KeepWorld" true)
  (bind _returnvalue_2 (AddComponent|AddAudioComponent false))
  (Variables|Default|SetSpeaker _returnvalue_2))

(fn ConstructionScript)

(fn ReceiveNewWaves
  (params (Array :type Array%20of%20BP%20Wave%20Object%20References))
  (for _array_element Array
    (Utilities|Array|AddUnique (Variables|Default|GetCurrentWaves) _array_element)))

(fn StopReceivingWaves
  (params (Array :type Array%20of%20BP%20Wave%20Object%20References))
  (for _array_element Array
    (Utilities|Array|RemoveItem (Variables|Default|GetCurrentWaves) _array_element)))

(fn UpdateScreen
  (Default|EventUpdate (Variables|Default|GetWaveScreen) (Variables|Default|GetCurrentWaves)))

(fn PlayWavesAudio
  (for _array_element (Variables|Default|GetCurrentWaves)
    (Utilities|Array|Add (LocalVariables|GetFrequencies) (* (Variables|/Game/Blueprints/Core/Wave/BP_Wave.BP_Wave_C|GetFrequency _array_element) 1e+02))
    (Utilities|Array|Add (LocalVariables|GetAmplitudes) (Variables|/Game/Blueprints/Core/Wave/BP_Wave.BP_Wave_C|GetAmplitude _array_element)))
  (Class|AudioParameterControllerInterface|SetFloatArrayParameter (Variables|Default|GetSpeaker) "HarmonicMultipliers" (LocalVariables|GetFrequencies)))