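; BP_Android is a simple AI enemy that carries an attached wave transmitter and can be disabled by waves from other transmitters.
; Pawn sensing sets the hasSeenPlayer blackboard key, cleared by a retriggerable delay after the last sighting.
; It collects foreign waves, ignoring its own, and dies when their overlapped frequency reaches a threshold.
; Death updates the blackboard, fires OnDeathTriggers, ragdolls the mesh and deactivates the transmitter.
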(event OnSeePawn(PawnSensing)
  (params (Pawn :type Pawn%20Object%20Reference))
  (if (Variables|Default|GetisActive)
    (Utilities|Casting|CastToBP_ThirdPersonCharacter Pawn)
    (AI|Components|Blackboard|SetValueasBool (AI|GetBlackboard (AI|GetAIController self)) (Utilities|Name|MakeLiteralName "hasSeenPlayer") true)
    (Utilities|FlowControl|RetriggerableDelay 4.0))
  (AI|Components|Blackboard|SetValueasBool (AI|GetBlackboard (AI|GetAIController self)) (Utilities|Name|MakeLiteralName "hasSeenPlayer") false))

(event Custom|Event%20Die
  (Utilities|FlowControl|DoOnce false
    (:Completed
      (Variables|Default|SetisActive false)
      (|UpdateBlackboard)
      (CallFunction|OnDeath)
      (CallFunction|ActivateRagdoll)
      (Components|Activation|SetActive (Variables|Default|GetTransmittingArea) false false)
      (Default|EventDeactivate (Variables|Default|GetAs%20BP%20Transmitter)))))

(event Event
  (params (Waves :type Array%20of%20BP%20Wave%20Object%20References) (Transmitter :type BP%20Transmitter%20Object%20Reference))
  (if (not (== Transmitter (Variables|Default|GetAs%20BP%20Transmitter)))
    (CallFunction|ReceiveWaves Waves Transmitter)
    (bind _should_disable_ (CallFunction|CheckDisableFrequency))
    (if _should_disable_
      (CallFunction|EventDie))))

(event EventStopReceiving
  (params (Waves :type Array%20of%20BP%20Wave%20Object%20References) (Transmitter :type Actor%20Object%20Reference))
  (if (not (== (Variables|Default|GetAs%20BP%20Transmitter) Transmitter))
    (CallFunction|StopReceivingWaves Waves Transmitter)))

(event EventBeginPlay
  (bind _asbp_attachable_transmitter (Utilities|Casting|CastToBP_AttachableTransmitter (Variables|/Script/Engine.ChildActorComponent|GetChildActor (Variables|Default|GetTransmitter))))
  (Variables|Default|SetAs%20BP%20Transmitter _asbp_attachable_transmitter)
  (Default|EventInit (Variables|Default|GetAs%20BP%20Transmitter) (Transformation|GetRelativeTransform (Variables|Default|GetTransmittingArea)) (Variables|Default|GetInitial%20Waves) (Utilities|Array|MakeArray self)))

(fn ConstructionScript)

(fn OnDeath
  (for _array_element (Variables|Default|GetOnDeathTriggers)
    (Class|BPITriggerable|Trigger(Message) _array_element)))

(fn ReceiveWaves
  (params (Waves :type Array%20of%20BP%20Wave%20Object%20References) (Transmitter :type Object%20Object%20Reference))
  (for _array_element Waves
    (Utilities|Array|AddUnique (Variables|Default|GetReceivingWaves) _array_element)))

(fn StopReceivingWaves
  (params (Waves :type Array%20of%20BP%20Wave%20Object%20References) (Transmitter :type Object%20Object%20Reference))
  (for _array_element Waves
    (Utilities|Array|RemoveItem (Variables|Default|GetReceivingWaves) _array_element)))

(fn CheckDisableFrequency
  (bind _frequency (CallFunction|OverlapWaves (Variables|Default|GetReceivingWaves)))
  (return (>= _frequency (* (Variables|Default|GetDisableFrequencyThreshold) 1e+02))))

(fn ActivateRagdoll
  (bind _mesh (Variables|Character|GetMesh))
  (Audio|Components|Audio|Stop (Variables|Character|GetMesh))
  (Class|SkeletalMeshComponent|SetAllBodiesSimulatePhysics (Variables|Character|GetMesh) true)
  (Physics|SetSimulatePhysics _mesh true)
  (Class|PrimitiveComponent|WakeAllRigidBodies _mesh))