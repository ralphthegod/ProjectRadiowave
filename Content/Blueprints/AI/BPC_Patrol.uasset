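; BPC_Patrol is an AI patrol Blueprint that hands out the next indicator along a patrol path.
; GetNextIndicator returns the PathIndicators entry at CurrentIndicatorIndex, then advances the stored index.
; A modulo by the array length wraps the index to the start, so successive calls cycle the path in a loop.
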(fn GetNextIndicator
  (LocalVariables|SetIndicator (Utilities|Array|Get(acopy) (Variables|Default|GetPath%20Indicators) (Variables|Default|GetCurrent%20Indicator%20Index)))
  (Variables|Default|SetCurrent%20Indicator%20Index (Math|Integer|%(Integer) (+ (Variables|Default|GetCurrent%20Indicator%20Index) 1) (Utilities|Array|Length (Variables|Default|GetPath%20Indicators))))
  (return (LocalVariables|GetIndicator)))