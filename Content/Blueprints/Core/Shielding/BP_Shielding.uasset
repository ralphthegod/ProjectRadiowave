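; BP_Shielding is an interactable "Radio Shielding" actor that moves 100 units down when triggered.
; BeginPlay sets the text on its InteractionLabel widget, and Highlight and Unhighlight toggle that label and the mesh's custom depth.
; Trigger stores start and end locations, then a Timeline lerps the actor between them without sweep.
; Untrigger is empty, and the destroy logic is disconnected.
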(event EventBeginPlay
  (bind _asui_info_on_screen (Utilities|Casting|CastToUI_InfoOnScreen (UserInterface|GetUserWidgetObject (Variables|Default|GetInteraction%20Label))))
  (bind _output_get (Variables|Default|SetAs%20UI%20Info%20On%20Screen _asui_info_on_screen))
  (Default|EventSetText _output_get "Radio Shielding" "" (Utilities|Array|MakeArray)))

(event EventHighlight
  (Rendering|SetVisibility (Variables|Default|GetInteraction%20Label) true false)
  (Rendering|SetRenderCustomDepth (Variables|Default|GetStaticMesh) true))

(event EventUnhighlight
  (Rendering|SetVisibility (Variables|Default|GetInteraction%20Label) false false)
  (Rendering|SetRenderCustomDepth (Variables|Default|GetStaticMesh) false))

(event EventTrigger
  (bind _self self)
  (bind _self_2 self)
  (bind _returnvalue (Transformation|GetActorLocation _self))
  (Variables|Default|SetStartingPoint _returnvalue)
  (Variables|Default|SetEndPoint (- _returnvalue "0.000000,0.000000,100.000000"))
  (bind _newtrack_0 (Timeline|Timeline PlayFromStart)
    (:Update
      (Utilities|IsValid _self_2
        (:Is%20Valid
          (Transformation|SetActorLocation _self_2 (Math|Vector|Lerp(Vector) (Variables|Default|GetStartingPoint) (Variables|Default|GetEndPoint) _newtrack_0) false false))))))

(event EventUntrigger)

(fn ConstructionScript)