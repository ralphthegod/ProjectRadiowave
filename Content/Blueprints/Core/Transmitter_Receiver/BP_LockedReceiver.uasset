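; BP_LockedReceiver is a receiver puzzle actor that unlocks when incoming waves combine to a matching frequency and amplitude.
; At BeginPlay it spawns a screen on a socket and shows the target derived by overlapping its initial unlock waves.
; Received waves are added to or removed from a set, and each addition triggers the match check.
; A highlight label offers Analyze, which flags the receiver and returns its received waves.
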(event Custom|Event%20Unlock
  (Default|EventUnlock (Variables|Default|GetScreen)))

(event EventBeginPlay
  (bind _returnvalue (Game|SpawnActorfromClass "/Game/Blueprints/Core/Transmitter_Receiver/Receivers/LevelDoor/BP_LockedReceiverScreen.BP_LockedReceiverScreen_C" (Math|Conversions|ToTransform(Vector) "0, 0, 0") "Undefined" "MultiplyWithRoot" 0 0))
  (bind _output_get (Variables|Default|SetScreen _returnvalue))
  (Transformation|AttachComponentToComponent _output_get (Variables|Default|GetScreenSocket) "None" "SnapToTarget" "KeepRelative" "KeepWorld" true)
  (bind __waves (CallFunction|GetWavesfromStruct (Variables|Default|GetInitialUnlockWaves) self))
  (bind _output_get_2 (Variables|Default|SetWaves __waves))
  (bind (_frequency _amplitude) (CallFunction|OverlapWaves _output_get_2))
  (Default|EventShow (Variables|Default|GetScreen) _frequency _amplitude)
  (CallFunction|InitInteraction))

(event Event
  (params (Waves :type Array%20of%20BP%20Wave%20Object%20References) (Transmitter :type BP%20Transmitter%20Object%20Reference))
  (CallFunction|AddReceivingWaves Waves)
  (bind (_frequency _amplitude) (CallFunction|OverlapWaves (Variables|Default|GetReceivingWaves)))
  (bind (_frequency_2 _amplitude_2) (CallFunction|OverlapWaves (Variables|Default|GetWaves)))
  (if (and (== _frequency _frequency_2) (== _amplitude _amplitude_2))
    (CallFunction|EventUnlock)))

(event EventStopReceiving
  (params (Waves :type Array%20of%20BP%20Wave%20Object%20References) (Transmitter :type BP%20Transmitter%20Object%20Reference))
  (CallFunction|RemoveReceivingWaves Waves))

(event EventUnhighlight
  (Rendering|SetVisibility (Variables|Default|GetInteraction%20Label) false false))

(event EventHighlight
  (Rendering|SetVisibility (Variables|Default|GetInteraction%20Label) true false))

(fn ConstructionScript)

(fn RemoveReceivingWaves
  (params (Array :type Array%20of%20BP%20Wave%20Object%20References))
  (for _array_element Array
    (Utilities|Array|RemoveItem (Variables|Default|GetReceivingWaves) _array_element)))

(fn AddReceivingWaves
  (params (Array :type Array%20of%20BP%20Wave%20Object%20References))
  (for _array_element Array
    (Utilities|Array|AddUnique (Variables|Default|GetReceivingWaves) _array_element)))

(fn InitInteraction
  (bind _asui_info_on_screen (Utilities|Casting|CastToUI_InfoOnScreen (UserInterface|GetUserWidgetObject (Variables|Default|GetInteraction%20Label))))
  (bind _output_get (Variables|Default|SetAs%20UI%20Info%20On%20Screen _asui_info_on_screen))
  (Default|EventSetText _output_get "" "Receiver" (Utilities|Array|MakeArray (Utilities|Struct|MakeS_InteractionEntry "LMB" "Analyze"))))

(fn Analyze
  (Variables|Default|SetisAnalyzed? true)
  (return (Variables|Default|GetReceivingWaves)))