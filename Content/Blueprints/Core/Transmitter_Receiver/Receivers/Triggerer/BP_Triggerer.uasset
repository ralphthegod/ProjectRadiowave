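; BP_Triggerer is a receiver in the Transmitter/Receiver system that relays an unlock into trigger messages for other objects.
; On its first unlock event, a DoOnce gate calls TriggerEverything, which sends TriggerMessage to each element of the ToTrigger array.
; Highlight and Unhighlight extend the parent behavior by toggling custom depth rendering on the Cube component.
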(event EventHighlight
  (|CallParentFunction)
  (Rendering|SetRenderCustomDepth (Variables|Default|GetCube) true))

(event EventUnhighlight
  (|CallParentFunction)
  (Rendering|SetRenderCustomDepth (Variables|Default|GetCube) false))

(event EventEventUnlock
  (Utilities|FlowControl|DoOnce false
    (:Completed
      (CallFunction|TriggerEverything))))

(fn ConstructionScript)

(fn TriggerEverything
  (for _array_element (Variables|Default|GetToTrigger)
    (Class|BPITriggerable|Trigger(Message) _array_element)))