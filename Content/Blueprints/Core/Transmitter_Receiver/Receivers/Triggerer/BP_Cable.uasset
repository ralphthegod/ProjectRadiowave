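; BP_Cable is a receiver in the transmitter/receiver system: a cable with a power LED that lights when triggered.
; BeginPlay creates a dynamic material for the LED, switches it off and labels the on-screen info widget "Cable".
; Trigger sets the material's On/Off parameter to lit, with no path to turn it off again.
; Highlight and Unhighlight toggle the cube's custom depth rendering and the label's visibility.
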(event EventBeginPlay
  (bind _returnvalue (Rendering|Material|CreateDynamicMaterialInstance (Variables|Default|GetLED) 0 "/Game/Materials/LED/MI_PowerLED.MI_PowerLED" "None" :!class /Script/Engine.PrimitiveComponent))
  (bind _output_get (Variables|Default|SetLEDMaterial _returnvalue))
  (Rendering|Material|SetScalarParameterValue _output_get "On/Off" 0.0 :!class /Script/Engine.MaterialInstanceDynamic)
  (CallFunction|InitInteraction))

(event EventTrigger
  (Rendering|Material|SetScalarParameterValue (Variables|Default|GetLEDMaterial) "On/Off" 1.0 :!class /Script/Engine.MaterialInstanceDynamic))

(event EventUnhighlight
  (Rendering|SetRenderCustomDepth (Variables|Default|GetCube) false)
  (Rendering|SetVisibility (Variables|Default|GetInteraction%20Label) false false))

(event EventHighlight
  (Rendering|SetRenderCustomDepth (Variables|Default|GetCube) true)
  (Rendering|SetVisibility (Variables|Default|GetInteraction%20Label) true false))

(fn ConstructionScript)

(fn InitInteraction
  (bind _asui_info_on_screen (Utilities|Casting|CastToUI_InfoOnScreen (UserInterface|GetUserWidgetObject (Variables|Default|GetInteraction%20Label))))
  (bind _output_get (Variables|Default|SetAs%20UI%20Info%20On%20Screen _asui_info_on_screen))
  (Default|EventSetText _output_get "Cable" "" (Utilities|Array|MakeArray)))