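; Screen for a locked level-door receiver that displays the frequency and amplitude it requires and signals when it is unlocked.
; BeginPlay creates a dynamic wave-screen material on Plane1 and caches the widget from Screen.
; Show sends both values to the widget, then clears the material's numbered wave parameters and writes one BP_Wave built from them, with frequency divided by 100.
; Unlock forwards the event to the widget.
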(event Custom|Event%20Show
  (params (Required%20Freq :type Float%20%28double-precision%29) (Required%20Amp :type Float%20%28double-precision%29))
  (CallFunction|ShowRequiredFrequencies Required%20Freq Required%20Amp))

(event Custom|Event%20Unlock
  (Default|EventUnlock (Variables|Default|GetLockedReceiverInterface)))

(event EventBeginPlay
  (bind _returnvalue (Rendering|Material|CreateDynamicMaterialInstance (Variables|Default|GetPlane1) 0 "/Game/Blueprints/WaveScreen/MI_WaveScreen.MI_WaveScreen" "Screen" :!class /Script/Engine.PrimitiveComponent))
  (bind _output_get (Variables|Default|SetScreenMaterialInstance _returnvalue))
  (Rendering|Material|SetMaterial (Variables|Default|GetPlane1) 0 _output_get)
  (bind _asui_locked_receiver_screen (Utilities|Casting|CastToUI_LockedReceiverScreen (UserInterface|GetUserWidgetObject (Variables|Default|GetScreen))))
  (Variables|Default|SetLockedReceiverInterface _asui_locked_receiver_screen))

(fn ConstructionScript)

(fn ShowRequiredFrequencies
  (params (Freq :type Float%20%28double-precision%29) (Amp :type Float%20%28double-precision%29))
  (bind _lockedreceiverinterface (Variables|Default|GetLockedReceiverInterface))
  (Utilities|FlowControl|Sequence
    (:then_0
      (Utilities|IsValid _lockedreceiverinterface
        (:Is%20Valid
          (Default|EventShow _lockedreceiverinterface Freq Amp))))
    (:then_1
      (bind _returnvalue (Game|ConstructObjectfromClass "/Game/Blueprints/Core/Wave/BP_Wave.BP_Wave_C" (/ Freq 1e+02) Amp))
      (CallFunction|ClearMaterialInstanceParameters)
      (CallFunction|SetMaterialInstanceParameters (Utilities|Array|MakeArray _returnvalue)))))

(fn ClearMaterialInstanceParameters
  (for _index (range 1 30)
    (Rendering|Material|SetScalarParameterValue (Variables|Default|GetScreenMaterialInstance) (Utilities|String|StringToName (Utilities|String|ToString(Text) (Utilities|Text|FormatText "Frequency{i}" _index))) 0.0 :!class /Script/Engine.MaterialInstanceDynamic)
    (Rendering|Material|SetScalarParameterValue (Variables|Default|GetScreenMaterialInstance) (Utilities|String|StringToName (Utilities|String|ToString(Text) (Utilities|Text|FormatText "Amplitude{i}" _index))) 0.0 :!class /Script/Engine.MaterialInstanceDynamic)))

(fn SetMaterialInstanceParameters
  (params (Waves :type Array%20of%20BP%20Wave%20Object%20References))
  (for (_array_element _array_index) Waves
    (Rendering|Material|SetScalarParameterValue (Variables|Default|GetScreenMaterialInstance) (Utilities|String|StringToName (Utilities|String|ToString(Text) (Utilities|Text|FormatText "Frequency{i}" (+ _array_index 1)))) (Variables|/Game/Blueprints/Core/Wave/BP_Wave.BP_Wave_C|GetFrequency _array_element) :!class /Script/Engine.MaterialInstanceDynamic)
    (Rendering|Material|SetScalarParameterValue (Variables|Default|GetScreenMaterialInstance) (Utilities|String|StringToName (Utilities|String|ToString(Text) (Utilities|Text|FormatText "Amplitude{i}" (+ _array_index 1)))) (Variables|/Game/Blueprints/Core/Wave/BP_Wave.BP_Wave_C|GetAmplitude _array_element) :!class /Script/Engine.MaterialInstanceDynamic)))