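; BP_LevelDoor is a sci-fi level door, built as a receiver in the transmitter/receiver system, that opens when unlocked.
; Wave reception, stop-receiving and unlock events defer to the parent class, and unlock then passes through a DoOnce to play the door's skeletal mesh animation without looping.
; Highlight and unhighlight toggle custom depth rendering on that mesh.
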(event EventBeginPlay
  (|CallParentFunction))

(event EventEventUnlock
  (|CallParentFunction)
  (Utilities|FlowControl|DoOnce false
    (:Completed
      (CallFunction|UnlockDoor))))

(event Event
  (params (Waves :type Array%20of%20BP%20Wave%20Object%20References) (Transmitter :type BP%20Transmitter%20Object%20Reference))
  (|CallParentFunction Waves Transmitter))

(event EventStopReceiving
  (params (Waves :type Array%20of%20BP%20Wave%20Object%20References) (Transmitter :type BP%20Transmitter%20Object%20Reference))
  (|CallParentFunction Waves Transmitter))

(event EventUnhighlight
  (|CallParentFunction)
  (Rendering|SetRenderCustomDepth (Variables|Default|GetSkeletalMesh) false))

(event EventHighlight
  (|CallParentFunction)
  (Rendering|SetRenderCustomDepth (Variables|Default|GetSkeletalMesh) true))

(fn ConstructionScript)

(fn UnlockDoor
  (Components|Animation|PlayAnimation (Variables|Default|GetSkeletalMesh) "/Game/Meshes/Door/Cooper_SCIFI_DOOR11_Anim.Cooper_SCIFI_DOOR11_Anim" false))