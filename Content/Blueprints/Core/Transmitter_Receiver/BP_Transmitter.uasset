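; Transmitter actor that broadcasts waves to receivers inside its transmitting area, with highlighting, an info label and an Analyze function that returns its waves.
; Activation builds waves from initial data and nudges the area's transform to refresh overlaps, which track BPI_Receiver actors.
; Each tick, a line trace to each receiver sends the waves, or stops them if BP_Shielding is hit.
; Deactivation stops all receivers and clears the waves.
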(event OnComponentEndOverlap(TransmittingArea)
  (params (OverlappedComponent :type Primitive%20Component%20Object%20Reference) (OtherActor :type Actor%20Object%20Reference) (OtherComp :type Primitive%20Component%20Object%20Reference) (OtherBodyIndex :type Integer))
  (Utilities|ShouldIgnore? OtherComp)
  (bind _asbpi_receiver (Utilities|Casting|CastToBPI_Receiver OtherActor))
  (if (not (Utilities|Array|ContainsItem (Variables|Default|GetIgnore%20Actors) _asbpi_receiver))
    (if (Variables|Default|GetisActive?)
      (Utilities|Array|RemoveItem (Variables|Default|GetOverlappingReceivers) OtherActor)
      (Class|BPIReceiver|StopReceiving(Message) OtherActor (Variables|Default|GetWaves) self))))

(event OnComponentBeginOverlap(TransmittingArea)
  (params (OverlappedComponent :type Primitive%20Component%20Object%20Reference) (OtherActor :type Actor%20Object%20Reference) (OtherComp :type Primitive%20Component%20Object%20Reference) (OtherBodyIndex :type Integer) (bFromSweep :type Boolean) (SweepResult :type Hit%20Result%20Structure%20%28by%20ref%29))
  (Utilities|ShouldIgnore? OtherComp)
  (bind _asbpi_receiver (Utilities|Casting|CastToBPI_Receiver OtherActor))
  (if (not (Utilities|Array|ContainsItem (Variables|Default|GetIgnore%20Actors) _asbpi_receiver))
    (Utilities|Array|AddUnique (Variables|Default|GetOverlappingReceivers) OtherActor)))

(event Custom|Event%20Activate
  (Variables|Default|SetisActive? true)
  (CallFunction|InitializeWaves)
  (CallFunction|ResetTransmittingArea))

(event Custom|Event%20Deactivate
  (bind _overlappingreceivers (Variables|Default|GetOverlappingReceivers))
  (Variables|Default|SetisActive? false)
  (for _array_element _overlappingreceivers
    (Class|BPIReceiver|StopReceiving(Message) _array_element (Variables|Default|GetWaves) self))
  (Utilities|Array|Clear _overlappingreceivers)
  (Variables|/Script/Engine.PrimitiveComponent|SetbGenerateOverlapEvents (Variables|Default|GetTransmittingArea) false)
  (Utilities|Array|Clear (Variables|Default|GetWaves)))

(event EventTick
  (params (DeltaSeconds :type Float%20%28single-precision%29))
  (CallFunction|CheckSignalObstruction))

(event EventUnhighlight
  (Rendering|SetVisibility (Variables|Default|GetInteraction%20Label) false false)
  (for _array_element (Variables|Default|GetHighlightableMeshes)
    (Rendering|SetRenderCustomDepth _array_element false)))

(event EventStopAnalyzing)

(event EventBeginPlay
  (CallFunction|GetHighlightableComponents)
  (bind _asui_info_on_screen (Utilities|Casting|CastToUI_InfoOnScreen (UserInterface|GetUserWidgetObject (Variables|Default|GetInteraction%20Label))))
  (bind _output_get (Variables|Default|SetAs%20UI%20Info%20On%20Screen _asui_info_on_screen))
  (Default|EventSetText _output_get (Variables|Default|GetName) "Transmitter" (Variables|Default|GetInteractionEntries))
  (if (Variables|Default|GetisActive?)
    (Utilities|FlowControl|Delay 0.2)
    (CallFunction|EventActivate)))

(event EventHighlight
  (Rendering|SetVisibility (Variables|Default|GetInteraction%20Label) true false)
  (for _array_element (Variables|Default|GetHighlightableMeshes)
    (Rendering|SetRenderCustomDepth _array_element true)))

(fn ConstructionScript)

(fn CheckSignalObstruction
  (if (Variables|Default|GetisActive?)
    (for _array_element (Variables|Default|GetOverlappingReceivers)
      (LocalVariables|SetCurrentReceiver _array_element)
      (bind _outhit (Collision|LineTraceByChannel (Transformation|GetWorldLocation (Variables|Default|GetSignalSourcePoint)) (Transformation|GetActorLocation (LocalVariables|GetCurrentReceiver)) "TraceTypeQuery1" false 0 "None"))
      (Utilities|Casting|CastToBP_Shielding (.HitActor (Collision|BreakHitResult _outhit))
        (:then
          (Class|BPIReceiver|StopReceiving(Message) (LocalVariables|GetCurrentReceiver) (Variables|Default|GetWaves) self))
        (:CastFailed
          (Class|BPIReceiver|Receive(Message) (LocalVariables|GetCurrentReceiver) (Variables|Default|GetWaves) self))))))

(fn GetHighlightableComponents
  (for _array_element (Components|GetChildrenComponents (Variables|Default|GetDefaultSceneRoot) true)
    (bind _asstatic_mesh_component (Utilities|Casting|CastToStaticMeshComponent _array_element))
    (Utilities|Array|AddUnique (Variables|Default|GetHighlightableMeshes) _asstatic_mesh_component)))

(fn InitializeWaves
  (bind __waves (CallFunction|GetWavesfromStruct (Variables|Default|GetInitial%20Waves) self))
  (Variables|Default|SetWaves __waves))

(fn ResetTransmittingArea
  (Variables|/Script/Engine.PrimitiveComponent|SetbGenerateOverlapEvents (Variables|Default|GetTransmittingArea) true)
  (LocalVariables|SetOriginal%20Transform (Transformation|GetRelativeTransform (Variables|Default|GetTransmittingArea)))
  (Transformation|SetRelativeTransform (Variables|Default|GetTransmittingArea) (Math|Conversions|ToTransform(Vector) "0, 0, 0") false false)
  (Transformation|SetRelativeTransform (Variables|Default|GetTransmittingArea) (LocalVariables|GetOriginal%20Transform) false false))

(fn Analyze
  (Variables|Default|SetisAnalyzed? true)
  (return (Variables|Default|GetWaves)))