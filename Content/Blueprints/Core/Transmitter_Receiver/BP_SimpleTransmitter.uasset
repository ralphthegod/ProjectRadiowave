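; BP_SimpleTransmitter is a transmitter Blueprint that shows its active state on a power LED and lists an "Analyze" interaction on LMB.
; BeginPlay creates a dynamic material instance for the LED and registers the interaction entry.
; EventActivate and EventDeactivate toggle the LED through the material's "On/Off" scalar parameter, then defer to the parent class for the remaining behavior.
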(event EventBeginPlay
  (bind _returnvalue (Rendering|Material|CreateDynamicMaterialInstance (Variables|Default|GetPowerLED) 0 "/Game/Materials/LED/MI_PowerLED.MI_PowerLED" "None" :!class /Script/Engine.PrimitiveComponent))
  (Variables|Default|SetLEDMaterial _returnvalue)
  (Utilities|Array|Add (Variables|Default|GetInteractionEntries) (Utilities|Struct|MakeS_InteractionEntry "LMB" "Analyze"))
  (|CallParentFunction))

(event EventEventActivate
  (Rendering|Material|SetScalarParameterValue (Variables|Default|GetLEDMaterial) "On/Off" 1.0 :!class /Script/Engine.MaterialInstanceDynamic)
  (|CallParentFunction))

(event EventEventDeactivate
  (Rendering|Material|SetScalarParameterValue (Variables|Default|GetLEDMaterial) "On/Off" 0.0 :!class /Script/Engine.MaterialInstanceDynamic)
  (|CallParentFunction))

(fn ConstructionScript
  (|CallParentFunction))