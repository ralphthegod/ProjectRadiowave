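; A draggable variant of a simple transmitter that adds a right mouse button "Drag" interaction entry.
; Drag enables physics on the main mesh and stores its world rotation, which Tick reapplies while physics simulates to keep the orientation locked.
; Drop waits on a retriggerable delay, then wakes the bodies and disables physics only if the mesh is not simulating.
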(event EventBeginPlay
  (Utilities|Array|Add (Variables|Default|GetInteractionEntries) (Utilities|Struct|MakeS_InteractionEntry "RMB" "Drag"))
  (|CallParentFunction))

(event EventTick
  (params (DeltaSeconds :type Float%20%28single-precision%29))
  (|CallParentFunction DeltaSeconds)
  (if (Physics|IsSimulatingPhysics (Variables|Default|GetMainMesh) "None")
    (Transformation|SetWorldRotation (Variables|Default|GetMainMesh) (Variables|Default|GetForced%20Rotation) false false)))

(event EventDrag
  (Physics|SetSimulatePhysics (Variables|Default|GetMainMesh) true)
  (Variables|Default|SetForced%20Rotation (Transformation|GetWorldRotation (Variables|Default|GetMainMesh))))

(event EventDrop
  (bind _mainmesh (Variables|Default|GetMainMesh))
  (Utilities|FlowControl|RetriggerableDelay 4.0)
  (if (not (Physics|IsSimulatingPhysics (Variables|Default|GetMainMesh) "None"))
    (Class|PrimitiveComponent|WakeAllRigidBodies _mainmesh)
    (Physics|SetSimulatePhysics _mainmesh false)))

(fn ConstructionScript
  (|CallParentFunction))